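; BP_PlantSpawner is a plant or tree actor that holds fruit and drops it when interacted with.
; Shortly after BeginPlay, it spawns a BP_Fruit at each child of SpawnPoints; the random 1–3 check always passes.
; Interact releases the stored fruits by enabling their tick, physics and gravity, with HasSpawned preventing repeat drops.
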(event `self.ReceiveBeginPlay`
  (`KismetSystemLibrary.Delay` 0.2)
  (`self.load fruit in tree`))

(event `load fruit in tree`
  ;[1 1 1] Load Fruit in Tree
  (`KismetArrayLibrary.Array_Append` (`self.spawnList`) (`SceneComponent.GetChildrenComponents` (`self.spawnPoints`) false))
  (for _array_element (`self.spawnList`)
    (if (> (`KismetMathLibrary.RandomIntegerInRange` 1 3) 0)
      (bind _returnvalue (`|SpawnActorFromClass` "/Game/Fruit/BP_Fruit.BP_Fruit_C" (`KismetMathLibrary.MakeTransform` (`SceneComponent.K2_GetComponentLocation` _array_element)) "Undefined" "MultiplyWithRoot" null null))
      (`KismetArrayLibrary.Array_Add` (`self.spawnedPoints`) _array_element)
      (`KismetArrayLibrary.Array_Add` (`self.spawnedFruits`) _returnvalue))))

(event `Spawn Fruit`
  ;[1 1 1] spawn fruit
  (for _array_element (`self.spawnedFruits`)
    (`self.SetActorTickEnabled` _array_element true)
    (bind _fruitmesh (`/Game/Fruit/BP_Fruit.fruitmesh` _array_element))
    (`PrimitiveComponent.SetSimulatePhysics` _fruitmesh true)
    (`PrimitiveComponent.SetEnableGravity` _fruitmesh true)
    (set `self.hasSpawned` true)))

(event `/Game/Character/Character_Blueprints/BPI_InteractInterface.Interact`
  (if (not (`self.hasSpawned`))
    (`self.Spawn Fruit`)))

(fn `UserConstructionScript`)