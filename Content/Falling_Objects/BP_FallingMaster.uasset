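; BP_FallingMaster is a falling object that shakes and then drops when an actor tagged "player" enters its trigger box.
; The overlap plays a timeline that offsets the actor on Z by the shake track scaled by ShakeAmplitude.
; A Delay of ShakeDuration, fed by the timeline's update, then enables physics simulation on the static mesh and switches its collision to physics-only.
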(event `self.Box.OnComponentBeginOverlap`
  (params (OverlappedComponent :type "PrimitiveComponent Object Reference") (OtherActor :type "Actor Object Reference") (OtherComp :type "PrimitiveComponent Object Reference") (OtherBodyIndex :type Integer) (bFromSweep :type Boolean) (SweepResult :type "HitResult Structure (by ref)"))
  (bind _staticmesh (`self.StaticMesh`))
  (if (`self.ActorHasTag` OtherActor "player")
    (bind (_direction _shake_track) (`Timeline|Shake Timeline`)
      (:`Update`
        (`self.K2_AddActorWorldOffset` (`KismetMathLibrary.MakeVector` 0.0 0.0 (* _shake_track (`self.shakeAmplitude`))))
        (`KismetSystemLibrary.Delay` (`self.shakeDuration`))
        (`PrimitiveComponent.SetSimulatePhysics` _staticmesh true)
        (`PrimitiveComponent.SetCollisionEnabled` _staticmesh "PhysicsOnly")))))

(fn `UserConstructionScript`)