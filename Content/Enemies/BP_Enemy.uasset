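; BP_Enemy is an enemy character that constantly walks forward, reacting to obstacles and ledges.
; WallDetector begin-overlap and LedgeDetector end-overlap both feed RespondToObstacle, which turns it around for EnemyBlocker-tagged actors.
; Otherwise it jumps if JumpOverObstacles is set, or turns around.
; Any damage sets Health to Damage minus Health (operands reversed from usual subtraction), destroying the actor at zero or below.
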(event `self.ReceiveAnyDamage`
  (params (Damage :type "Float (single-precision)") (DamageType :type "DamageType Object Reference") (InstigatedBy :type "Controller Object Reference") (DamageCauser :type "Actor Object Reference"))
  ;[1 1 1] Damage Enemy
  (bind _output_get (set `self.Health` (- Damage (`self.Health`))))
  (if (<= _output_get 0)
    (`self.K2_DestroyActor`)))

(event `self.ReceiveTick`
  (params (DeltaSeconds :type "Float (single-precision)"))
  (`self.AddMovementInput` (`self.GetActorForwardVector`)))

(event `self.Wall Detector.OnComponentBeginOverlap`
  (params (OverlappedComponent :type "PrimitiveComponent Object Reference") (OtherActor :type "Actor Object Reference") (OtherComp :type "PrimitiveComponent Object Reference") (OtherBodyIndex :type Integer) (bFromSweep :type Boolean) (SweepResult :type "HitResult Structure (by ref)"))
  (`self.Respond To Obstacle` OtherActor))

(event `Turn Character`
  ;[1 1 1] Turn Character Around
  (`self.K2_SetActorRotation` (`KismetMathLibrary.ComposeRotators` (`self.K2_GetActorRotation`) (struct :`Yaw` 180.0))))

(event `self.Ledge Detector.OnComponentEndOverlap`
  (params (OverlappedComponent :type "PrimitiveComponent Object Reference") (OtherActor :type "Actor Object Reference") (OtherComp :type "PrimitiveComponent Object Reference") (OtherBodyIndex :type Integer))
  (`self.Respond To Obstacle` OtherActor))

(event `Respond To Obstacle`
  (params (`Other Actor` :type "Actor Object Reference"))
  ;[1 1 1] Determine Response to Detect Obstacle
  (if (`self.ActorHasTag` `Other Actor` "EnemyBlocker")
    (`self.Turn Character` :!label _label)
    (elif (`self.JumpOverObstacles`)
      (`self.Jump`)
      (else
        (goto _label)))))

(fn `UserConstructionScript`)