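; Checkpoint actor that registers itself as the ActiveCheckpoint on GameMode_MAIN.
; One flagged as StartingCheckPoint claims that slot on BeginPlay.
; Any checkpoint takes it over when a BP_CharacterMAIN overlaps it, with no check for whether it is already active.
; Both paths print a "Checkpoint Activated" message.
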(event `self.ReceiveBeginPlay`
  (if (`self.StartingCheckPoint`)
    (bind _asgame_mode_main (cast `/Game/GameMode_MAIN` (`GameplayStatics.GetGameMode`)))
    (set `/Game/GameMode_MAIN.ActiveCheckpoint` self _asgame_mode_main)
    (`KismetSystemLibrary.PrintString` "Checkpoint Activated")))

(event `self.ReceiveActorBeginOverlap`
  (params (OtherActor :type "Actor Object Reference"))
  (cast `/Game/Character/Character_Blueprints/BP_CharacterMAIN` OtherActor)
  (bind _asgame_mode_main (cast `/Game/GameMode_MAIN` (`GameplayStatics.GetGameMode`)))
  (set `/Game/GameMode_MAIN.ActiveCheckpoint` self _asgame_mode_main)
  (`KismetSystemLibrary.PrintString` "Checkpoint Activated"))

(fn `UserConstructionScript`)