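; BP_Fruit is a collectible fruit pickup that hovers above surfaces.
; Each Tick, a downward line trace pushes the physics mesh along the hit normal, harder when closer to the surface, and applies linear and angular damping.
; Sphere overlap by a "player"-tagged actor increments FruitCount on the player's BP_CharacterMAIN and destroys the fruit.
; A droptimer event, intended for damage drops, destroys it after a short delay.
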(event `droptimer`
  ;[1 1 1] time until fruit despawns after damage
  (`KismetSystemLibrary.Delay` 5.0)
  (`self.K2_DestroyActor`))

(event `self.ReceiveTick`
  (params (DeltaSeconds :type "Float (single-precision)"))
  (bind _fruitmesh (`self.fruitmesh`))
  (bind _returnvalue (`SceneComponent.K2_GetComponentLocation` (`self.fruitmesh`)))
  ;[1 1 1] Fruit Float Function
  (bind (_outhit _returnvalue_2) (`KismetSystemLibrary.LineTraceSingle` _returnvalue (- _returnvalue (`KismetMathLibrary.MakeVector` 0.0 0.0 (`self.Trace Length`))) "TraceTypeQuery1"))
  (if _returnvalue_2
    (bind (_bblockinghit _binitialoverlap _time _distance _location _impactpoint _normal _impactnormal) (`GameplayStatics.BreakHitResult` _outhit))
    (`PrimitiveComponent.AddForce` _fruitmesh (* _impactnormal (`KismetMathLibrary.Lerp` 500000.0 0.0 (/ (`KismetMathLibrary.VSize` (- _location _returnvalue)) (`self.Trace Length`)))) "None" false)
    (`PrimitiveComponent.SetLinearDamping` _fruitmesh (`self.Linear Damping`))
    (`PrimitiveComponent.SetAngularDamping` (`self.fruitmesh`) (`self.Angular Damping`))))

(event `self.Sphere.OnComponentBeginOverlap`
  (params (OverlappedComponent :type "PrimitiveComponent Object Reference") (OtherActor :type "Actor Object Reference") (OtherComp :type "PrimitiveComponent Object Reference") (OtherBodyIndex :type Integer) (bFromSweep :type Boolean) (SweepResult :type "HitResult Structure (by ref)"))
  ;[1 1 1] pickup fruit on overlap
  (if (`self.ActorHasTag` OtherActor "player")
    (bind _asbp_character_main (cast `/Game/Character/Character_Blueprints/BP_CharacterMAIN` (`GameplayStatics.GetPlayerCharacter` 0)))
    (set `/Game/Character/Character_Blueprints/BP_CharacterMAIN.Fruit Count` (+ (`/Game/Character/Character_Blueprints/BP_CharacterMAIN.Fruit Count` _asbp_character_main) 1) _asbp_character_main)
    (`self.K2_DestroyActor`)))

(fn `UserConstructionScript`)